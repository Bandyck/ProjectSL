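; BP_Spider_mutant is a mutant spider character Blueprint that plays a random animation montage, apparently as an asset-pack showcase.
; BeginPlay waits a fixed delay and a random delay around a multi-input DoOnce, then picks one of seven attack, death, hit or turn montages.
; The DoOnce is reset afterward, but nothing loops back to replay.
; Tick is empty, and a walk-speed setter and second montage call are disconnected.
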(event EventBeginPlay
  (Utilities|FlowControl|Delay 3.0)
  (|DoOnceMultiInput :!label _label
    (:A%20Out
      _)
    (:Reset%20Out
      _))
  (Utilities|FlowControl|Delay (Math|Random|RandomFloatinRange 1.0 4.0))
  (Utilities|FlowControl|Sequence
    (:then_0
      (Animation|PlayAnimMontage (Utilities|Array|Get(acopy) (Utilities|Array|MakeArray "/Game/Monster_pack_01BD/Spider_mutant/animations/montages/anim_atack_1_Montage.anim_atack_1_Montage" "/Game/Monster_pack_01BD/Spider_mutant/animations/montages/anim_attack_02_Montage.anim_attack_02_Montage" "/Game/Monster_pack_01BD/Spider_mutant/animations/montages/anim_attack_Montage.anim_attack_Montage" "/Game/Monster_pack_01BD/Spider_mutant/animations/montages/anim_dye_Montage.anim_dye_Montage" "/Game/Monster_pack_01BD/Spider_mutant/animations/montages/anim_hit_Montage.anim_hit_Montage" "/Game/Monster_pack_01BD/Spider_mutant/animations/montages/anim_turn_left_Montage.anim_turn_left_Montage" "/Game/Monster_pack_01BD/Spider_mutant/animations/montages/anim_turn_right_Montage.anim_turn_right_Montage" 0) (Math|Random|RandomIntegerinRange 0 6)) 1.0 "None")
      (goto _label Reset%20In))))

(event Collision|EventActorBeginOverlap
  (params (OtherActor :type Actor%20Object%20Reference)))

(event EventTick
  (params (DeltaSeconds :type Float%20%28single-precision%29)))

(fn ConstructionScript)